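; BP_Pillar is a pillar that can be activated once, fading in a glow and broadcasting its activation.
; BeginPlay creates a dynamic material instance from M_PillarActivated on the Pillar component.
; ActivatePillar uses a boolean guard to start the glow and call OnPillarActivated a single time.
; Tick then eases GlowAlpha toward full with FInterpTo at GlowSpeed and writes it to the material parameter.
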(event Custom|ActivatePillar
  ;[1 1 1] Pillars can only be activated once thanks to the Branch check
  (if (not (Variables|Default|GetIsActivated?))
    (Variables|Default|SetIsActivated? true)
    (Variables|Default|SetGlowAlpha 0.0)
    (Variables|Default|SetTargetGlowAlpha 1.0)
    (Variables|Default|SetIsGlowing? true)
    (Default|CallOnPillarActivated)))

(event EventBeginPlay
  ;[1 1 1] Setting Base Colour
  (bind _returnvalue (Rendering|Material|CreateDynamicMaterialInstance (Variables|Default|GetPillar) 0 "/Game/Static/3DAliveAssets/AlivePillar/M_PillarActivated.M_PillarActivated" "" :!class /Script/Engine.PrimitiveComponent))
  (Variables|Default|SetDynMatPillar _returnvalue))

(event EventTick
  (params (DeltaSeconds :type Float%20%28single-precision%29))
  ;[1 1 1] Colour change logic for activated pillars
  (if (Variables|Default|GetIsGlowing?)
    (bind _output_get (Variables|Default|SetGlowAlpha (Math|Interpolation|FInterpTo (Variables|Default|GetGlowAlpha) (Variables|Default|GetTargetGlowAlpha) DeltaSeconds (Variables|Default|GetGlowSpeed))))
    (Rendering|Material|SetScalarParameterValue (Variables|Default|GetDynMatPillar) "GlowAlpha" _output_get :!class /Script/Engine.MaterialInstanceDynamic)))

(fn ConstructionScript)