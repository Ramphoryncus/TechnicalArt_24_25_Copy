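; Endgame gyroscopic portal whose three rings and central sphere spin on Tick until every pillar is activated.
; BeginPlay stores their start rotations and binds to each BP_Pillar's activation dispatcher to count activations.
; At the total, each part eases home via RInterpTo, then the sphere is hidden and NS_Portal spawns at a hardcoded location.
; A BP_Charger entering EndGameBox shows the outro widget, then loads the main menu after a delay.
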(event OnComponentBeginOverlap(EndGameBoxCollision)
  (params (OverlappedComponent :type Primitive%20Component%20Object%20Reference) (OtherActor :type Actor%20Object%20Reference) (OtherComp :type Primitive%20Component%20Object%20Reference) (OtherBodyIndex :type Integer) (bFromSweep :type Boolean) (SweepResult :type Hit%20Result%20Structure%20%28by%20ref%29))
  ;[1 1 1] Endgame collision to Outro widget
  (Utilities|Casting|CastToBP_Charger OtherActor)
  (bind _returnvalue (UserInterface|CreateWidget "/Game/Static/UI/OutroCharger3.OutroCharger3_C"))
  (UserInterface|Viewport|AddtoViewport _returnvalue 0)
  (Utilities|FlowControl|Delay 7.0)
  (Game|OpenLevel(byObjectReference) "/Game/Dynamic/Maps/MainMenuMap.MainMenuMap"))

(event Custom|PillarActivated
  ;[1 1 1] Incremental Pillar activation count to activate stop rotation
  (Math|Integer|IncrementInt (Variables|Default|GetActivatedPillars)
    (:%20%20
      (if (== (Variables|Default|GetTotalPillars) (Variables|Default|GetActivatedPillars))
        (Variables|Default|SetPortalReturnToStartRotation true)))))

(event EventBeginPlay
  (Utilities|FlowControl|Sequence
    (:then_0
      ;[1 1 1] Getting start rotation
      (Variables|Default|SetOuterStartRotation (Transformation|GetWorldRotation (Variables|Default|GetAlive_GyroscopicOuterRing)))
      (Variables|Default|SetMiddleStartRotation (Transformation|GetWorldRotation (Variables|Default|GetAlive_GyroscopicMiddleRing)))
      (Variables|Default|SetInnerStartRotation (Transformation|GetWorldRotation (Variables|Default|GetAlive_GyroscopicInnerRing)))
      (Variables|Default|SetSphereStartRotation (Transformation|GetWorldRotation (Variables|Default|GetAlive_GyroscopicSphere))))
    (:then_1
      ;[1 1 1] BP_Pillar event dispatcher bound to Custom Event Pillar Activated
      (bind _outactors (Actor|GetAllActorsOfClass "/Game/Dynamic/Blueprints/BP_Pillar.BP_Pillar_C"))
      (for _array_element _outactors
        (bind _asbp_pillar (Utilities|Casting|CastToBP_Pillar _array_element))
        (EventDispatchers|BindEventtoOnPillarActivated _asbp_pillar (EventDispatchers|CreateEvent :!event Custom|PillarActivated))))))

(event EventTick
  (params (DeltaSeconds :type Float%20%28single-precision%29))
  (bind _alive_gyroscopicouterring (Variables|Default|GetAlive_GyroscopicOuterRing))
  (bind _alive_gyroscopicmiddlering (Variables|Default|GetAlive_GyroscopicMiddleRing))
  (bind _alive_gyroscopicinnerring (Variables|Default|GetAlive_GyroscopicInnerRing))
  (bind _alive_gyroscopicsphere (Variables|Default|GetAlive_GyroscopicSphere))
  (bind _alive_gyroscopicsphere_2 (Variables|Default|GetAlive_GyroscopicSphere))
  (bind _alive_gyroscopicsphere_3 (Variables|Default|GetAlive_GyroscopicSphere))
  (if (Variables|Default|GetPortalReturnToStartRotation)
    ;[1 1 1] Stop Rotating and RETURN to START Rotation on ALL 4 Pillars Activated
    (Variables|Default|SetOuterRingRotationSpeed 0.0)
    (Variables|Default|SetMiddleRingRotationSpeed 0.0)
    (Variables|Default|SetInnerRingRotationSpeed 0.0)
    (Variables|Default|SetSphereRotationSpeed 0.0)
    (Transformation|SetWorldRotation _alive_gyroscopicouterring (Math|Interpolation|RInterpTo (Transformation|GetWorldRotation _alive_gyroscopicouterring) (Variables|Default|GetOuterStartRotation) DeltaSeconds 0.25) false false)
    (Transformation|SetWorldRotation _alive_gyroscopicmiddlering (Math|Interpolation|RInterpTo (Transformation|GetWorldRotation _alive_gyroscopicmiddlering) (Variables|Default|GetMiddleStartRotation) DeltaSeconds 0.5) false false)
    (Transformation|SetWorldRotation _alive_gyroscopicinnerring (Math|Interpolation|RInterpTo (Transformation|GetWorldRotation _alive_gyroscopicinnerring) (Variables|Default|GetInnerStartRotation) DeltaSeconds 0.75) false false)
    (Transformation|SetWorldRotation _alive_gyroscopicsphere_3 (Math|Interpolation|RInterpTo (Transformation|GetWorldRotation _alive_gyroscopicsphere_3) (Variables|Default|GetSphereStartRotation) DeltaSeconds 1.0) false false)
    ;[1 1 1] Destroy the sphere spawn Niagara Portal and sphere location
    (if (Utilities|Operators|EqualEqual (Transformation|GetWorldRotation _alive_gyroscopicsphere) (Variables|Default|GetSphereStartRotation) 0.2)
      (Utilities|IsValid _alive_gyroscopicsphere
        (:Is%20Valid
          (Utilities|FlowControl|Delay 2.0)
          (Rendering|SetVisibility _alive_gyroscopicsphere_2 false false)
          (Collision|SetCollisionEnabled _alive_gyroscopicsphere_2 "NoCollision")
          (Variables|Default|SetSphereRotationSpeed 0.0)
          (Niagara|SpawnSystematLocation "/Game/Dynamic/Niagara/NS_Portal.NS_Portal" "16793.514874,-37.627226,-1233.034566" "0, 0, 0" "1.000000,1.000000,1.000000" false))))
    (else
      ;;[1 1 1] Rotators
      (Transformation|AddLocalRotation (Variables|Default|GetAlive_GyroscopicOuterRing) (Math|Rotator|MakeRotator 0.0 0.0 (Variables|Default|GetOuterRingRotationSpeed)) false false)
      (Transformation|AddLocalRotation (Variables|Default|GetAlive_GyroscopicMiddleRing) (Math|Rotator|MakeRotator 0.0 (Variables|Default|GetMiddleRingRotationSpeed) 0.0) false false)
      (Transformation|AddLocalRotation (Variables|Default|GetAlive_GyroscopicInnerRing) (Math|Rotator|MakeRotator 0.0 0.0 (Variables|Default|GetInnerRingRotationSpeed)) false false)
      (Transformation|AddLocalRotation (Variables|Default|GetAlive_GyroscopicSphere) (Math|Rotator|MakeRotator 0.0 (Variables|Default|GetSphereRotationSpeed) 0.0) false false))))

(fn ConstructionScript)