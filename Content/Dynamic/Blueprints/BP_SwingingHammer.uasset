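; BP_SwingingHammer is a hammer obstacle that spins continuously and knocks back any BP_Charger it hits.
; Tick yaws the hammer mesh by a frame-rate-independent HammerRotationSpeed.
; On component hit, it launches the charger along the mesh's forward vector scaled by HitStrength, overriding existing velocity.
; Timeline swings, timer-driven RotateHammer and alternative hit-direction calculations remain as disconnected, unused experiments.
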(event OnComponentHit(SM_SwingingHammer)
  (params (HitComponent :type Primitive%20Component%20Object%20Reference) (OtherActor :type Actor%20Object%20Reference) (OtherComp :type Primitive%20Component%20Object%20Reference) (NormalImpulse :type Vector :default "0, 0, 0") (Hit :type Hit%20Result%20Structure%20%28by%20ref%29))
  ;[1 1 1] Hammer Time (tm MC Hammer) with adjustable HitStrength
  (bind _asbp_charger (Utilities|Casting|CastToBP_Charger OtherActor))
  (Character|LaunchCharacter _asbp_charger (* (Math|Vector|GetForwardVector (Variables|Default|GetSM_SwingingHammer)) (Variables|Default|GetHitStrength)) true true))

(event OnComponentBeginOverlap(SM_SwingingHammer)
  (params (OverlappedComponent :type Primitive%20Component%20Object%20Reference) (OtherActor :type Actor%20Object%20Reference) (OtherComp :type Primitive%20Component%20Object%20Reference) (OtherBodyIndex :type Integer) (bFromSweep :type Boolean) (SweepResult :type Hit%20Result%20Structure%20%28by%20ref%29))
  ;[1 1 1] It's an old code but it checks out
)

(event OnComponentHit(Box)
  (params (HitComponent :type Primitive%20Component%20Object%20Reference) (OtherActor :type Actor%20Object%20Reference) (OtherComp :type Primitive%20Component%20Object%20Reference) (NormalImpulse :type Vector :default "0, 0, 0") (Hit :type Hit%20Result%20Structure%20%28by%20ref%29))
  ;[1 1 1] It's an old code but it checks out
)

(event EventBeginPlay)

(event Collision|EventActorBeginOverlap
  (params (OtherActor :type Actor%20Object%20Reference)))

(event EventTick
  (params (DeltaSeconds :type Float%20%28single-precision%29))
  (Transformation|AddLocalRotation (Variables|Default|GetSM_SwingingHammer) (Math|Rotator|MakeRotator 0.0 0.0 (* DeltaSeconds (Variables|Default|GetHammerRotationSpeed))) false false))

(fn ConstructionScript)

(fn RotateHammer
  (Transformation|AddLocalRotation (Variables|Default|GetSM_SwingingHammer) (Math|Rotator|MakeRotator 0.0 0.0 (Variables|Default|GetHammerFunctionRotationSpeed)) false false))